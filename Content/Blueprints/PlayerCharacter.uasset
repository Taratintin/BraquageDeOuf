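; Player character for a two-plane side-scroller with grappling hook, charged melee attack, gold total and HUD.
; Horizontal input walks or runs along Y, while holding Z shifts the character between clamped front and back X planes.
; Space traces upward to attach a cable and disable gravity; impulses drive climbing and sideways jumps off the rope.
; Tick updates planes, hook lift and charge, which slows movement; full-charge release calls an unfinished attack stub.
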(event `self.ReceiveTick`
  (params (DeltaSeconds :type "Float (single-precision)"))
  (`|ExecutionSequence`
    (:`then_0`
      (`self.PlaneMovement`))
    (:`then_1`
      (`self.ChargeAttack`))
    (:`then_2`
      (if (`self.hooked`)
        (`CharacterMovementComponent.AddImpulse` (`self.CharacterMovement`) (0.0 0.0 12.0) true)))))

(event `self.ReceiveBeginPlay`
  (`self.ResetGrapple`)
  (bind _returnvalue (`|CreateWidget` "/Game/Blueprints/Main_HUD.Main_HUD_C" (`GameplayStatics.GetPlayerController` 0)))
  (`UserWidget.AddToViewport` _returnvalue 0))

(event `InputAxis|Horizontal`
  (params (AxisValue :type "Float (single-precision)"))
  ;[1 1 1] Movement
  (if (`self.hooked`)
    (`MovementComponent.StopMovementImmediately` (`self.CharacterMovement`))
    (elif (`self.isWalking`)
      (`self.AddMovementInput` (0.0 -1.0 0.0) (/ AxisValue 4.0))
      (else
        (`self.AddMovementInput` (0.0 -1.0 0.0) AxisValue)))))

(event `InputAxis|Vertical`
  (params (AxisValue :type "Float (single-precision)"))
  ;[1 1 1] Vertical Movement while hooked
  (if (`self.hooked`)
    (`CharacterMovementComponent.AddImpulse` (`self.CharacterMovement`) (`KismetMathLibrary.MakeVector` 0.0 0.0 (+ AxisValue 20.0)) true)))

(event `Key|LeftShift`
  (params (Key :type "Key Structure"))
  ;[1 1 1] Movement
  (:`Pressed`
    (set `self.isWalking` true))
  (:`Released`
    (set `self.isWalking` false)))

(event `Key|D`
  (params (Key :type "Key Structure"))
  ;[1 1 1] Jump off the rope to one or the other side
  (:`Pressed`
    (if (`self.hooked`)
      (`CharacterMovementComponent.AddImpulse` (`self.CharacterMovement`) (0.0 -750.0 450.0) true)
      (set `self.hooked` false :!label _label)
      (`PrimitiveComponent.SetEnableGravity` (`self.CapsuleComponent`) true)
      (`self.ResetGrapple`))))

(event `InputAction|Matraque`
  (params (Key :type "Key Structure"))
  ;[1 1 1] This manages the Charging Attack state
  (:`Pressed`
    (set `self.isCharging` true))
  (:`Released`
    (if (>= (`self.chargePercent`) 100.0)
      (`self.UseAttack`))
    (set `self.chargePercent` 0.0)
    (set `self.isCharging` false)
    (set `self.isWalking` false)
    (`KismetSystemLibrary.PrintString` "Sweet Release")))

(event `Key|Q`
  (params (Key :type "Key Structure"))
  ;[1 1 1] Jump off the rope to one or the other side
  (:`Pressed`
    (if (`self.hooked`)
      (`CharacterMovementComponent.AddImpulse` (`self.CharacterMovement`) (0.0 750.0 450.0) true)
      (goto _label))))

(event `Key|Z`
  (params (Key :type "Key Structure"))
  ;[1 1 1] Define target plane (front or back)
  (:`Pressed`
    (set `self.targetBackPlane` true))
  (:`Released`
    (set `self.targetBackPlane` false)))

(event `Key|SpaceBar`
  (params (Key :type "Key Structure"))
  (bind _returnvalue (`self.K2_GetActorLocation` self))
  (:`Pressed`
    (if (`self.hooked`)
      (goto _label)
      (else
        ;[1 1 1] Linetrace to see if there's a surface to hook to, and to "Get" the surface touched
        (bind (_outhit _returnvalue_2) (`KismetSystemLibrary.LineTraceSingleForObjects` _returnvalue (`KismetMathLibrary.MakeVector` (.x _returnvalue) (.y _returnvalue) (+ (.z _returnvalue) 10000.0)) (`|MakeArray` "ObjectTypeQuery1" "ObjectTypeQuery2" :!type "EObjectTypeQuery Enum")))
        (if _returnvalue_2
          (set `self.hooked` true)
          (`PrimitiveComponent.SetEnableGravity` (`self.CapsuleComponent`) false)
          (`CableComponent.SetAttachEndTo` (`self.Grapple`) (`.HitActor` (`GameplayStatics.BreakHitResult` _outhit)) "None" "None")
          (`SceneComponent.SetVisibility` (`self.Grapple`) true false))))))

(fn `AddGold`
  (params (NewParam :type Integer))
  (set `self.TotalGold` (+ (`self.TotalGold`) NewParam)))

(fn `ChargeAttack`
  (if (and (`self.isCharging`) (< (`self.chargePercent`) 100.0))
    (bind _output_get (set `self.chargePercent` (+ (`self.chargePercent`) (/ 100.0 (* (`self.secsToAttack`) 30.0)))))
    (`KismetSystemLibrary.PrintString` (`KismetStringLibrary.Conv_DoubleToString` _output_get) true true (struct :`G` 0.66 :`B` 1.0 :`A` 1.0) 0.5)
    (set `self.isWalking` true)))

(fn `PlaneMovement`
  (bind _x (.x (`self.K2_GetActorLocation`)))
  (if (not (`self.hooked`))
    ;[1 1 1] Is the player trying to go to the back?
    (if (`self.targetBackPlane`)
      ;[1 1 1] Moves the player according to its location
      (if (> _x -130.0)
        (`self.AddMovementInput` (-10.0 0.0 0.0) 1.0 true)
        (else
          ;[1 1 1] If the player went too far "backwards", then teleport him at -130
          (`self.K2_SetActorLocation` (`KismetMathLibrary.MakeVector` -130.0 (.y (`self.K2_GetActorLocation`)) (.z (`self.K2_GetActorLocation`))))))
      (elif (< _x 0.0)
        (`self.AddMovementInput` (10.0 0.0 0.0) 1.0 true)
        (else
          ;[1 1 1] If the player when too far "forward", then teleports him at 0
          (`self.K2_SetActorLocation` (`KismetMathLibrary.MakeVector` 0.0 (.y (`self.K2_GetActorLocation`)) (.z (`self.K2_GetActorLocation`))))))))
  (return))

(fn `ResetGrapple`
  (bind _grapple (`self.Grapple`))
  (`SceneComponent.SetVisibility` _grapple false false)
  (set `CableComponent.CableLength` 0.0 _grapple)
  (set `CableComponent.CableWidth` 8.0 _grapple)
  (set `CableComponent.EndLocation` (0.0 0.0 0.0) _grapple))

(fn `UseAttack`
  (`KismetSystemLibrary.PrintString` "WATTA!!")
  (bind _outactors (`GameplayStatics.GetAllActorsOfClass` (`self.ennemyClass`)))
  (set `self.NewVar_0` _outactors)
  (if (`PrimitiveComponent.IsOverlappingActor` (`self.Knocker`) null)
    _))

(fn `UserConstructionScript`)