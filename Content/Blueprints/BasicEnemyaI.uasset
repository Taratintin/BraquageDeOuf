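; A basic enemy Blueprint that patrols between two points, PointA and PointB, using an InterpToMovement component.
; The Construction Script builds the relative control points from those two variables.
; On each movement reversal, a FlipFlop alternates the capsule's world rotation between two opposite orientations to turn the enemy around.
; The capsule overlap event is empty, so the enemy has no contact logic here.
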(event `self.InterpToMovement.OnInterpToReverse`
  (params (ImpactResult :type "HitResult Structure (by ref)") (Time :type "Float (single-precision)"))
  (bind _capsulecomponent (`self.CapsuleComponent`))
  (`/Engine/EditorBlueprintResources/StandardMacros.FlipFlop`
    (:`A`
      (`SceneComponent.K2_SetWorldRotation` _capsulecomponent (struct :`Yaw` 180.0) false false))
    (:`B`
      (`SceneComponent.K2_SetWorldRotation` :`self` _capsulecomponent))))

(event `self.CapsuleComponent.OnComponentBeginOverlap`
  (params (OverlappedComponent :type "PrimitiveComponent Object Reference") (OtherActor :type "Actor Object Reference") (OtherComp :type "PrimitiveComponent Object Reference") (OtherBodyIndex :type Integer) (bFromSweep :type Boolean) (SweepResult :type "HitResult Structure (by ref)")))

(fn `UserConstructionScript`
  (set `InterpToMovementComponent.ControlPoints` (`|MakeArray` (make `InterpControlPoint` (`self.PointA`)) (make `InterpControlPoint` (`self.PointB`))) (`self.InterpToMovement`)))